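; A door Blueprint that swings open on trigger overlap, either freely or by consuming a key.
; Its Box checks the overlapping component's tag, then opens keyless non-switch doors directly; otherwise KeyName must be Got in MyGameInstance, which resets it to Default.
; OpenDoor clears SwitchDoor and drives the mesh's yaw with a timeline.
; The SetEventFinished override calls the parent, snaps the door open and disables trigger collision.
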(event `self.ReceiveBeginPlay`
  (`parent.ReceiveBeginPlay`))

(event `self.Box.OnComponentBeginOverlap`
  (params (OverlappedComponent :type "PrimitiveComponent Object Reference") (OtherActor :type "Actor Object Reference") (OtherComp :type "PrimitiveComponent Object Reference") (OtherBodyIndex :type Integer) (bFromSweep :type Boolean) (SweepResult :type "HitResult Structure (by ref)"))
  (if (`ActorComponent.ComponentHasTag` OtherComp "None")
    (if (and (== (`self.KeyName`) "None") (not (`self.Switch Door`)))
      (`self.Open Door`)
      (else
        (switch `/Game/Project/BluePrints/EN_KeyStatus` (`/Game/Project/BluePrints/BP_MyGameInstance.GetKeyStatus` (`self.MyGameInstance`) (`self.KeyName`))
          (:`NewEnumerator1`
            (`/Game/Project/BluePrints/BP_MyGameInstance.SaveKeyStatus` (`self.MyGameInstance`) (`self.KeyName`) "NewEnumerator0")
            (`self.Open Door`)))))))

(event `Open Door`
  (set `self.Switch Door` false)
  (bind (_direction _open_z) (`Timeline|Open`)
    (:`Update`
      (`SceneComponent.K2_SetRelativeRotation` (`self.STM_Door`) (`KismetMathLibrary.MakeRotator` 0.0 0.0 _open_z) false false))
    (:`Finished`
      (`self.SetEventFinished`))))

(fn `SetEventFinished`
  (`parent.SetEventFinished`)
  (set `self.Switch Door` false)
  (`SceneComponent.K2_SetRelativeRotation` (`self.STM_Door`) (struct :`Yaw` 90.0) false false)
  (`PrimitiveComponent.SetCollisionEnabled` (`self.Box`) "NoCollision"))

(fn `UserConstructionScript`)