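; AI controller that drives an enemy's behavior tree and tracks a player character through AI perception.
; On BeginPlay it initializes the BB_MyCharacter blackboard and runs BT_MyCharacter.
; Perception updates write the first stimulus's sensed state to bDiscovered for each updated actor.
; A sensed BP_MyCharacter is stored as TargetPlayer, and a lost stimulus clears that key.
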(event `self.ReceiveBeginPlay`
  (`self.UseBlackboard` "/Game/BB_MyCharacter.BB_MyCharacter")
  (`self.RunBehaviorTree` "/Game/BT_MyCharacter.BT_MyCharacter"))

(event `self.AIPerception.OnPerceptionUpdated`
  (params (UpdatedActors :type "Array of Actor Object Reference (by ref)"))
  (for _array_element UpdatedActors
    (bind _info (`AIPerceptionComponent.GetActorsPerception` (`self.AIPerception`) _array_element))
    (bind (_age _expirationage _strength _stimuluslocation _receiverlocation _tag _bsuccessfullysensed) (break `AIStimulus` (`|GetArrayItem` (`.LastSensedStimuli` (break `ActorPerceptionBlueprintInfo` _info)))))
    (`BlackboardComponent.SetValueAsBool` (`AIBlueprintHelperLibrary.GetBlackboard` null) "bDiscovered" _bsuccessfullysensed)
    (if _bsuccessfullysensed
      (bind _asbp_my_character (cast `/Game/Project/BluePrints/BP_MyCharacter` _array_element))
      (`BlackboardComponent.SetValueAsObject` (`AIBlueprintHelperLibrary.GetBlackboard` null) "TargetPlayer" _asbp_my_character)
      (else
        (`BlackboardComponent.SetValueAsObject` (`AIBlueprintHelperLibrary.GetBlackboard` null) "TargetPlayer" null)))))

(fn `UserConstructionScript`)